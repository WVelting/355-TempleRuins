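; Crate actor that bursts into a shower of physics macaroni when destroyed.
; A Trigger event destroys the actor, while AnyDamage subtracts from Health but does nothing when it reaches zero.
; On Destroyed, a loop spawns roughly 150 Macaroni_Blueprint actors at seeded random offsets around the crate with random rotations, launching each at high speed in a random direction.
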(event `/Game/Blueprints/Interfaces/TriggerableObject.Trigger`
  (`self.K2_DestroyActor`))

(event `self.ReceiveAnyDamage`
  (params (Damage :type "Float (single-precision)") (DamageType :type "DamageType Object Reference") (InstigatedBy :type "Controller Object Reference") (DamageCauser :type "Actor Object Reference"))
  (bind _output_get (set `self.health` (- (`self.health`) Damage)))
  (if (<= _output_get 0.0)
    _))

(event `self.ReceiveDestroyed`
  (for _ (range 151)
    (bind _returnvalue (`|SpawnActorFromClass` "/Game/Blueprints/Macaroni_Blueprint.Macaroni_Blueprint_C" (`KismetMathLibrary.MakeTransform` (+ (* (`KismetMathLibrary.RandomUnitVectorFromStream` (`self.Stream_0`)) 30.0) (`self.K2_GetActorLocation`)) (`KismetMathLibrary.RandomRotator` false)) "Undefined" "OverrideRootScale" (`self.GetOwner`) null))
    (`PrimitiveComponent.SetAllPhysicsLinearVelocity` (`StaticMeshActor.StaticMeshComponent` _returnvalue) (* (`KismetMathLibrary.RandomUnitVectorFromStream` (`self.Stream`)) 1600.0) false)))

(fn `UserConstructionScript`)