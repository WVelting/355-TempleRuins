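; Pressure plate that switches a linked actor on when something overlaps its box and off when the overlap ends.
; Overlap begin plays a timeline that lowers the button mesh, and overlap end reverses it.
; When the timeline finishes, its direction sets IsOff and sends TurnOn or TurnOff through the ToggleableObject interface.
; Overlaps act only if the linked actor is valid and implements that interface, with no filter on the overlapping actor.
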(event `self.Box.OnComponentBeginOverlap`
  (params (OverlappedComponent :type "PrimitiveComponent Object Reference") (OtherActor :type "Actor Object Reference") (OtherComp :type "PrimitiveComponent Object Reference") (OtherBodyIndex :type Integer) (bFromSweep :type Boolean) (SweepResult :type "HitResult Structure (by ref)"))
  (bind _actorscontrolledbythisactor (`self.ActorsControlledByThisActor`))
  (bind _actorscontrolledbythisactor_2 (`self.ActorsControlledByThisActor`))
  ;[1 1 1] Starts Event on Overlap with other Actors
  (`/Engine/EditorBlueprintResources/StandardMacros.IsValid` _actorscontrolledbythisactor
    (:`Is Valid`
      (if (`KismetSystemLibrary.DoesImplementInterface` _actorscontrolledbythisactor "/Game/Blueprints/Interfaces/ToggleableObject.ToggleableObject_C")
        ;[1 1 1] Handles On/Off Animation
        (bind (_direction _percent) (`Timeline|ButtonAnim` :!label _label)
          (:`Update`
            (`SceneComponent.K2_SetRelativeLocation` (`self.Button`) (`KismetMathLibrary.MakeVector` 0.0 0.0 (* _percent -3.0)) false false))
          (:`Finished`
            (switch `ETimelineDirection` _direction
              (:`Forward`
                ;[1 1 1] Sends Message to Toggleable Object
                (set `self.IsOff` false)
                (message `/Game/Blueprints/Interfaces/ToggleableObject.TurnOn` _actorscontrolledbythisactor_2))
              (:`Backward`
                (set `self.IsOff` true)
                (message `/Game/Blueprints/Interfaces/ToggleableObject.TurnOff` _actorscontrolledbythisactor_2)))))))))

(event `self.Box.OnComponentEndOverlap`
  (params (OverlappedComponent :type "PrimitiveComponent Object Reference") (OtherActor :type "Actor Object Reference") (OtherComp :type "PrimitiveComponent Object Reference") (OtherBodyIndex :type Integer))
  (bind _actorscontrolledbythisactor (`self.ActorsControlledByThisActor`))
  ;[1 1 1] Starts Event on Overlap with other Actors
  (`/Engine/EditorBlueprintResources/StandardMacros.IsValid` _actorscontrolledbythisactor
    (:`Is Valid`
      (if (`KismetSystemLibrary.DoesImplementInterface` _actorscontrolledbythisactor "/Game/Blueprints/Interfaces/ToggleableObject.ToggleableObject_C")
        (goto _label :!via `Reverse`)))))

(fn `UserConstructionScript`)