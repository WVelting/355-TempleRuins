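; Lever actor that the player toggles to switch one linked actor on or off.
; On interaction it checks that the linked actor is valid and implements the ToggleableObject interface, then plays or reverses the LeverAnim timeline based on IsOff.
; The timeline pitches the Mover component, and only when it finishes does it update IsOff and send the matching TurnOn or TurnOff message.
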(event `/Game/Blueprints/Interfaces/PlayerCanInteract.PlayerWantsToInteract`
  (params (Player :type "/Game/Blueprints/FirstPersonCharacter Object Reference"))
  (bind _otheractorscontrolledbythisactor (`self.OtherActorsControlledByThisActor`))
  (bind _otheractorscontrolledbythisactor_2 (`self.OtherActorsControlledByThisActor`))
  ;[1 1 1] Receives Input from Player Character
  (`/Engine/EditorBlueprintResources/StandardMacros.IsValid` _otheractorscontrolledbythisactor_2
    (:`Is Valid`
      (if (`KismetSystemLibrary.DoesImplementInterface` _otheractorscontrolledbythisactor_2 "/Game/Blueprints/Interfaces/ToggleableObject.ToggleableObject_C")
        ;[1 1 1] Handles On/Off Animation
        (if (`self.IsOff`)
          (bind (_direction _percent) (`Timeline|LeverAnim` :!label _label)
            (:`Update`
              (`SceneComponent.K2_SetRelativeRotation` (`self.Mover`) (`KismetMathLibrary.MakeRotator` 0.0 (* _percent 150.0)) false false))
            (:`Finished`
              (switch `ETimelineDirection` _direction
                (:`Forward`
                  ;[1 1 1] Sends Message to Toggleable Object
                  (set `self.IsOff` false)
                  (message `/Game/Blueprints/Interfaces/ToggleableObject.TurnOn` _otheractorscontrolledbythisactor))
                (:`Backward`
                  (set `self.IsOff` true)
                  (message `/Game/Blueprints/Interfaces/ToggleableObject.TurnOff` _otheractorscontrolledbythisactor)))))
          (else
            (goto _label :!via `Reverse`)))))))

(fn `UserConstructionScript`)