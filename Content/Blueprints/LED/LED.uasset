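; LED Blueprint that shows a red, green or blue state as a color on its static mesh.
; The construction script creates a dynamic material instance and calls ChangeLEDColor, which maps CurrentState to the LEDColor parameter.
; Trigger cycles CurrentState with a Select node but does not refresh the material.
; An equivalent Switch version and an event-graph ChangeLEDColor call are left unconnected.
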(event `/Game/Blueprints/Interfaces/TriggerableObject.Trigger`
  ;[1 1 1] Change State with Select
  (set `self.CurrentState` (select `/Game/Blueprints/LED/LEDColor` (`self.CurrentState`) :`NewEnumerator0` "NewEnumerator1" :`NewEnumerator1` "NewEnumerator2" :`NewEnumerator2` "NewEnumerator0" :!type "/Game/Blueprints/LED/LEDColor Enum")))

(fn `Change LED Color`
  ;[1 1 1] Update the material
  (`MaterialInstanceDynamic.SetVectorParameterValue` (`self.LED Material`) "LEDColor" (select `/Game/Blueprints/LED/LEDColor` (`self.CurrentState`) :`NewEnumerator0` (struct :`R` 1.0 :`A` 1.0) :`NewEnumerator1` (struct :`R` 0.089607 :`G` 1.0 :`A` 1.0) :`NewEnumerator2` (struct :`B` 1.0 :`A` 1.0) :!type "LinearColor Structure")))

(fn `UserConstructionScript`
  (bind _returnvalue (`PrimitiveComponent.CreateDynamicMaterialInstance` (`self.StaticMesh`) 0 "/Game/Blueprints/LED/LED_Mat.LED_Mat" "None"))
  (set `self.LED Material` _returnvalue)
  (`self.Change LED Color`))